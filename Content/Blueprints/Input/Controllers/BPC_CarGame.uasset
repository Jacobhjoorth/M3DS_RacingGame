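; Per-player controller for a car game with up to four players, covering menu car selection, readying up and game start.
; ConnecttoGame assigns a team colour and menu input, then a timer cycles the view through tagged cinematic cameras.
; Readying spawns and possesses the chosen car at that player's PlayerStart.
; Enhanced Input mapping contexts follow each phase, while car choice, ready state and quitting go through the GameMode's main menu widget.
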(event `self.ReceiveBeginPlay`
  (`WidgetBlueprintLibrary.SetInputMode_GameAndUIEx` self null)
  (bind _asgm_car_game (cast `/Game/Blueprints/GameRules/GM_CarGame` (`GameplayStatics.GetGameMode`)))
  (set `self.WB_MainMenu` (`/Game/Blueprints/GameRules/GM_CarGame.WB_MainMenu` _asgm_car_game)))

(event `EnhancedInput|/Game/Blueprints/Input/Actions/MyInputs/IA_NextCar`
  (params (ActionValue :type Boolean) (ElapsedSeconds :type "Float (double-precision)") (TriggeredSeconds :type "Float (double-precision)") (InputAction :type "InputAction Object Reference" :default "/Game/Blueprints/Input/Actions/MyInputs/IA_NextCar.IA_NextCar"))
  (:`Started`
    (`/Game/UI/WB_MainMenu.ChangeCar` (`self.WB_MainMenu`) (`self.PlayerIndex`) true)))

(event `EnhancedInput|/Game/Blueprints/Input/Actions/MyInputs/IA_PreviousCar`
  (params (ActionValue :type Boolean) (ElapsedSeconds :type "Float (double-precision)") (TriggeredSeconds :type "Float (double-precision)") (InputAction :type "InputAction Object Reference" :default "/Game/Blueprints/Input/Actions/MyInputs/IA_PreviousCar.IA_PreviousCar"))
  (:`Started`
    (`/Game/UI/WB_MainMenu.ChangeCar` (`self.WB_MainMenu`) (`self.PlayerIndex`) false)))

(event `EnhancedInput|/Game/Blueprints/Input/Actions/MyInputs/IA_Ready`
  (params (ActionValue :type Boolean) (ElapsedSeconds :type "Float (double-precision)") (TriggeredSeconds :type "Float (double-precision)") (InputAction :type "InputAction Object Reference" :default "/Game/Blueprints/Input/Actions/MyInputs/IA_Ready.IA_Ready"))
  (bind _returnvalue (pcsubsystem `EnhancedInputLocalPlayerSubsystem` (`GameplayStatics.GetPlayerController` (`self.PlayerIndex`))))
  (:`Started`
    (`/Engine/EditorBlueprintResources/StandardMacros.DoOnce` false
      (:`Completed`
        (set `self.bReady` true)
        (`self.SpawnAndPossess` (`self.PlayerIndex`))
        (`EnhancedInputSubsystemInterface.RemoveMappingContext` _returnvalue "/Game/Blueprints/Input/MappingContexts/IMC_Menu.IMC_Menu" (struct))
        (`EnhancedInputSubsystemInterface.AddMappingContext` _returnvalue "/Game/Blueprints/Input/MappingContexts/IMC_Ready.IMC_Ready" 0 (struct))
        (`/Game/UI/WB_MainMenu.ReadyPlayer` (`self.WB_MainMenu`) (`self.PlayerIndex`))))))

(event `EnhancedInput|/Game/Blueprints/Input/Actions/IA_ToggleCamera`
  (params (ActionValue :type Boolean) (ElapsedSeconds :type "Float (double-precision)") (TriggeredSeconds :type "Float (double-precision)") (InputAction :type "InputAction Object Reference" :default "/Game/Blueprints/Input/Actions/IA_ToggleCamera.IA_ToggleCamera")))

(event `/Game/Blueprints/Interfaces/BPI_StartGame.ConnectToGame`
  (params (PlayerIndex :type Integer))
  (bind _output_get (set `self.PlayerIndex` PlayerIndex))
  (`self.SetCarColor` _output_get)
  (`EnhancedInputSubsystemInterface.AddMappingContext` (pcsubsystem `EnhancedInputLocalPlayerSubsystem` (`GameplayStatics.GetPlayerController` (`self.PlayerIndex`))) "/Game/Blueprints/Input/MappingContexts/IMC_Menu.IMC_Menu" 100 (struct))
  (`self.SetOverlayEnabled` (`self.PlayerIndex`))
  (set `self.Tag` "1")
  (bind _returnvalue (`KismetSystemLibrary.K2_SetTimerDelegate` (delegate `ChangeCamera`) 5.0 (`self.bLoopingActive`)))
  (set `self.CinematicCameraTimer` _returnvalue)
  (`self.FindCinematicCamera`))

(event `ChangeCamera`
  (switch `int` (`self.CameraCount`)
    (:`0`
      (set `self.Tag` "2")
      (`/Engine/EditorBlueprintResources/StandardMacros.IncrementInt` (`self.CameraCount`)
        (:`  `
          _)))
    (:`1`
      (set `self.Tag` "3")
      (`/Engine/EditorBlueprintResources/StandardMacros.IncrementInt` (`self.CameraCount`)
        (:`  `
          _)))
    (:`2`
      (set `self.Tag` "4")
      (`/Engine/EditorBlueprintResources/StandardMacros.IncrementInt` (`self.CameraCount`)
        (:`  `
          _)))
    (:`3`
      (set `self.Tag` "1")
      (set `self.CameraCount` 0)))
  (`self.FindCinematicCamera`))

(event `/Game/Blueprints/Interfaces/BPI_StartGame.StartGame`
  (set `self.bLoopingActive` false)
  (`KismetSystemLibrary.K2_ClearAndInvalidateTimerHandle` (`self.CinematicCameraTimer`))
  (bind _returnvalue (`|CreateWidget` "/Game/UI/WB_StartGame.WB_StartGame_C"))
  (`UserWidget.AddToViewport` _returnvalue 0)
  (`EnhancedInputSubsystemInterface.AddMappingContext` (pcsubsystem `EnhancedInputLocalPlayerSubsystem` (`GameplayStatics.GetPlayerController` (`self.PlayerIndex`))) "/Game/Blueprints/Input/MappingContexts/IMC_Isometric.IMC_Isometric" 100 (struct))
  (`WidgetBlueprintLibrary.SetInputMode_GameOnly` self)
  (set `self.bShowMouseCursor` false))

(event `EnhancedInput|/Game/Blueprints/Input/Actions/MyInputs/IA_Quit`
  (params (ActionValue :type Boolean) (ElapsedSeconds :type "Float (double-precision)") (TriggeredSeconds :type "Float (double-precision)") (InputAction :type "InputAction Object Reference" :default "/Game/Blueprints/Input/Actions/MyInputs/IA_Quit.IA_Quit"))
  (:`Triggered`
    (`UserWidget.AddToViewport` (`self.WB_MainMenu`) 0)
    (`/Game/UI/WB_MainMenu.QuitGame` (`self.WB_MainMenu`) (`self.PlayerIndex`))))

(fn `FindCinematicCamera`
  (if (`self.bLoopingActive`)
    (bind _outactors (`GameplayStatics.GetAllActorsOfClassWithTag` "/Script/CinematicCamera.CineCameraActor" (`self.Tag`)))
    (bind _output (`|GetArrayItem` _outactors (`self.PlayerIndex`)))
    (`/Engine/EditorBlueprintResources/StandardMacros.IsValid` _output
      (:`Is Valid`
        (`self.SetViewTargetWithBlend` _output)))))

(fn `SpawnAndPossess`
  (params (PlayerIndex :type Integer))
  (`KismetSystemLibrary.K2_ClearAndInvalidateTimerHandle` (`self.CinematicCameraTimer`))
  (set `self.bLoopingActive` false)
  (bind _outactors (`GameplayStatics.GetAllActorsOfClass` "/Script/Engine.PlayerStart"))
  (`self.GetCarClass` (`|GetArrayItem` (`/Game/UI/WB_MainMenu.CarTypes` (`self.WB_MainMenu`)) PlayerIndex))
  (bind _returnvalue (`|SpawnActorFromClass` (`self.CarClass`) (`self.GetTransform` (`|GetArrayItem` _outactors PlayerIndex)) "AlwaysSpawn" "MultiplyWithRoot" null (`self.TeamColor`) null null))
  (`self.Possess` _returnvalue))

(fn `UserConstructionScript`)