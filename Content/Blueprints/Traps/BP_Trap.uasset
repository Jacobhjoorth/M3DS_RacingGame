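; Trap that launches a VehicleAdvPawn entering its trigger and moves its Road component along Z.
; Overlap calls Fling for a velocity-change mesh impulse from RandomValue, whose random-range nodes are unused as shown.
; The GoUp timeline drives the road's relative height, and a one-second timer reverses it.
; Fling also holds an unreached random branch for a negated impulse and prints a debug string.
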(event `self.Trigger.OnComponentBeginOverlap`
  (params (OverlappedComponent :type "PrimitiveComponent Object Reference") (OtherActor :type "Actor Object Reference") (OtherComp :type "PrimitiveComponent Object Reference") (OtherBodyIndex :type Integer) (bFromSweep :type Boolean) (SweepResult :type "HitResult Structure (by ref)"))
  (if (!= OtherActor self)
    (bind _asvehicle_adv_pawn (cast `/Game/Blueprints/Vehicles/Default/VehicleAdvPawn` OtherActor))
    (`self.Fling` _asvehicle_adv_pawn)
    (`KismetSystemLibrary.K2_SetTimerDelegate` (delegate `ReverseAnimation`) 1.0)
    (bind (_direction _z) (`Timeline|GoUp` :!label _label)
      (:`Update`
        (`SceneComponent.K2_SetRelativeLocation` (`self.Road`) (`KismetMathLibrary.MakeVector` 0.0 0.0 _z) false false)))))

(event `ReverseAnimation`
  (goto _label :!via `Reverse`))

(fn `Fling`
  (params (WhichCar :type "/Game/Blueprints/Vehicles/Default/VehicleAdvPawn Object Reference"))
  (bind (_x _y _z) (`self.RandomValue`))
  (`PrimitiveComponent.AddImpulse` (`WheeledVehiclePawn.Mesh` WhichCar) (`KismetMathLibrary.MakeVector` _x _y _z) "None" true)
  (`KismetSystemLibrary.PrintString` "fly"))

(fn `UserConstructionScript`)